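; Ambient crystal sphere VFX actor that reacts when the third-person character overlaps it.
; From BeginPlay, a timeline spins and moves the mesh, recreating its dynamic material and storing an unused InitialColor on every update.
; Overlap activates sparks and RotatingMovement while a second timeline lerps the point light and EmissiveColor parameter from a fixed blue-violet to NewColor.
; Leaving deactivates both components and reverses the color timeline.
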(event `self.ReceiveBeginPlay`
  (bind _sm_crystalsphere (`self.SM_CrystalSphere`))
  ;[0.1254 0 0.9583 1 49] Blueprint Ambiant: Animation sans interactions
  (bind (_direction _translation_z) (`Timeline|Timeline`)
    (:`Update`
      (`SceneComponent.K2_AddLocalRotation` _sm_crystalsphere (`KismetMathLibrary.MakeRotator` 0.4 0.3 0.8) false false)
      (`SceneComponent.K2_SetRelativeLocation` _sm_crystalsphere _translation_z false false)
      (bind _returnvalue (`PrimitiveComponent.CreateDynamicMaterialInstance` (`self.SM_CrystalSphere`) 0 null "None"))
      (set `self.DynamicMaterial` _returnvalue)
      (bind _returnvalue_2 (`MaterialInstanceDynamic.K2_GetVectorParameterValue` (`self.DynamicMaterial`) "Color"))
      (set `self.Initial Color` _returnvalue_2))))

(event `self.ReceiveActorBeginOverlap`
  (params (OtherActor :type "Actor Object Reference"))
  ;[0 1 0.05366 1 49] Blueprint interactif avec input
  (cast `/Game/ThirdPerson/Blueprints/BP_ThirdPersonCharacter` OtherActor)
  (`ActorComponent.Activate` (`self.NS_Sparks`) false)
  (`ActorComponent.Activate` (`self.RotatingMovement`) false)
  (bind (_direction _colorchangespeed) (`Timeline|Timeline_Lerp` :!label _label)
    (:`Update`
      (bind _returnvalue (`KismetMathLibrary.LinearColorLerp` (struct :`R` 0.201556 :`B` 1.0 :`A` 1.0) (`self.New color`) _colorchangespeed))
      (`LightComponent.SetLightColor` (`self.PointLight`) _returnvalue true)
      (`MaterialInstanceDynamic.SetVectorParameterValue` (`self.DynamicMaterial`) "EmissiveColor" _returnvalue))))

(event `self.ReceiveActorEndOverlap`
  (params (OtherActor :type "Actor Object Reference"))
  ;[0 1 0.05366 1 49] Blueprint interactif avec input
  (cast `/Game/ThirdPerson/Blueprints/BP_ThirdPersonCharacter` OtherActor)
  (`ActorComponent.Deactivate` (`self.NS_Sparks`))
  (`ActorComponent.Deactivate` (`self.RotatingMovement`))
  (goto _label :!via `Reverse`))

(fn `UserConstructionScript`)