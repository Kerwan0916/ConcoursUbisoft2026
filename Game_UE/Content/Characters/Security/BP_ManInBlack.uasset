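; BP_ManInBlack is a security character that patrols a route and can be stunned.
; On BeginPlay it casts its AI controller, passes it the PatrolRoute and starts patrol movement after a short delay, printing debug text if the cast fails.
; StunMIB sets IsStunned, calls a montage play and clears the flag after a timed delay, then rejoins the same path to request the next patrol point.
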(event `StunMIB`
  (set `self.bIsStunned` true)
  (`self.PlayAnimMontage` null)
  (`KismetSystemLibrary.Delay` 3.0)
  (set `self.bIsStunned` false)
  (if (not (`self.bIsStunned`)) :!label _label
    (`KismetSystemLibrary.Delay` 0.5)
    (`self.MoveToNextPatrolPoint` (stale `self.ReceiveBeginPlay` _asman_in_black_aicontroller))))

(event `self.ReceiveBeginPlay`
  (bind _returnvalue (`AIBlueprintHelperLibrary.GetAIController` null))
  (bind _asman_in_black_aicontroller (cast `` _returnvalue)
    (:`then`
      (set `/Game/Characters/Security/BP_ManInBlack.PatrolPoints` (`self.PatrolRoute`) _asman_in_black_aicontroller)
      (goto _label))
    (:`CastFailed`
      (`KismetSystemLibrary.PrintString` (`KismetSystemLibrary.GetClassDisplayName` (`GameplayStatics.GetObjectClass` _returnvalue)))
      (`KismetSystemLibrary.PrintString` "CAST FAILED!"))))

(fn `UserConstructionScript`)