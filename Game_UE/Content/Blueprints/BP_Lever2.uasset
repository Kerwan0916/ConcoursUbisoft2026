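; BP_Lever2 is an interactable lever that switches streamed lighting levels and registers its activation with BP_gameState.
; Its trigger zone enables input and shows a mesh only for player controller 1, without checking which actor overlaps.
; Interacting stops the sparks, destroys that mesh and plays a timeline that rotates the lever.
; Each timeline update requests loading Lvl_Lighting_02 and unloading its Off variant, and completion reports the lever index.
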(event `self.Interact`
  (`ActorComponent.Deactivate` (`self.NS_Sparks`))
  (`ActorComponent.K2_DestroyComponent` (`self.StaticMesh`))
  (bind (_direction _lever1) (`Timeline|Timeline`)
    (:`Update`
      (`SceneComponent.K2_SetRelativeRotation` (`self.Lever2`) (`KismetMathLibrary.RLerp` (struct :`Roll` -80.0) (struct :`Roll` 80.0) _lever1) false false)
      (`GameplayStatics.LoadStreamLevel` "Lvl_Lighting_02" true)
      (`GameplayStatics.UnloadStreamLevel` "Lvl_Lighting_02_Off"))
    (:`Finished`
      (set `self.IsActivated` true)
      (bind _asbp_game_state (cast `/Game/ThirdPerson/Blueprints/BP_gameState` (`GameplayStatics.GetGameState`)))
      (`/Game/ThirdPerson/Blueprints/BP_gameState.RegisterLeverActivate` _asbp_game_state (`self.LeverIndex`)))))

(event `self.ReceiveBeginPlay`
  (`ActorComponent.Activate` (`self.NS_Sparks`) false))

(event `self.TriggerZone.OnComponentBeginOverlap`
  (params (OverlappedComponent :type "PrimitiveComponent Object Reference") (OtherActor :type "Actor Object Reference") (OtherComp :type "PrimitiveComponent Object Reference") (OtherBodyIndex :type Integer) (bFromSweep :type Boolean) (SweepResult :type "HitResult Structure (by ref)"))
  (bind _returnvalue (`GameplayStatics.GetPlayerController` 1))
  (`/Engine/EditorBlueprintResources/StandardMacros.IsValid` _returnvalue
    (:`Is Valid`
      (`self.EnableInput` _returnvalue)
      (`SceneComponent.SetHiddenInGame` (`self.StaticMesh`) false false))))

(event `self.TriggerZone.OnComponentEndOverlap`
  (params (OverlappedComponent :type "PrimitiveComponent Object Reference") (OtherActor :type "Actor Object Reference") (OtherComp :type "PrimitiveComponent Object Reference") (OtherBodyIndex :type Integer))
  (bind _returnvalue (`GameplayStatics.GetPlayerController` 1))
  (`/Engine/EditorBlueprintResources/StandardMacros.IsValid` _returnvalue
    (:`Is Valid`
      (`self.DisableInput` _returnvalue)
      (`SceneComponent.SetHiddenInGame` (`self.StaticMesh`) true false))))

(fn `UserConstructionScript`)