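; BP_EscapeLever is an interactable escape lever that responds when activated from inside its trigger zone.
; Entering TriggerZone sets CanActivate, enables input for player controller 0 and prints an on-screen prompt; leaving clears the flag and disables input.
; IA_Interact checks the flag and only prints a freedom message, with no further escape logic.
; The overlap events do not filter which actor triggers them.
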(event `self.TriggerZone.OnComponentBeginOverlap`
  (params (OverlappedComponent :type "PrimitiveComponent Object Reference") (OtherActor :type "Actor Object Reference") (OtherComp :type "PrimitiveComponent Object Reference") (OtherBodyIndex :type Integer) (bFromSweep :type Boolean) (SweepResult :type "HitResult Structure (by ref)"))
  (set `self.bCanActivate` true)
  (`self.EnableInput` (`GameplayStatics.GetPlayerController` 0))
  (`KismetSystemLibrary.PrintText` "Press [A] to escape!" true false (struct :`G` 1.0 :`B` 0.139124 :`A` 1.0)))

(event `EnhancedInput|/Game/Input/Actions/IA_Interact`
  (params (ActionValue :type Boolean) (ElapsedSeconds :type "Float (double-precision)") (TriggeredSeconds :type "Float (double-precision)") (InputAction :type "InputAction Object Reference" :default "/Game/Input/Actions/IA_Interact.IA_Interact"))
  (:`Started`
    (if (`self.bCanActivate`)
      (`KismetSystemLibrary.PrintText` "You're free!" true false (struct :`R` 1.0 :`G` 0.01282 :`A` 1.0)))))

(event `self.TriggerZone.OnComponentEndOverlap`
  (params (OverlappedComponent :type "PrimitiveComponent Object Reference") (OtherActor :type "Actor Object Reference") (OtherComp :type "PrimitiveComponent Object Reference") (OtherBodyIndex :type Integer))
  (set `self.bCanActivate` false)
  (`self.DisableInput` (`GameplayStatics.GetPlayerController` 0)))

(fn `UserConstructionScript`)