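; BP_Key is a colored key pickup for a two-player game, added to the game state's inventory with E or the right gamepad face button.
; Overlapping either trigger enables input for both controllers, provided the second exists; one reveals a plane, the other starts area particles and a timeline fading emissive to the key's color.
; Pickup plays a burst effect, removes the mesh and destroys the actor after a delay.
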(event `self.B_TriggerZone.OnComponentBeginOverlap`
  (params (OverlappedComponent :type "PrimitiveComponent Object Reference") (OtherActor :type "Actor Object Reference") (OtherComp :type "PrimitiveComponent Object Reference") (OtherBodyIndex :type Integer) (bFromSweep :type Boolean) (SweepResult :type "HitResult Structure (by ref)"))
  (bind _returnvalue (`GameplayStatics.GetPlayerController` 1))
  (`/Engine/EditorBlueprintResources/StandardMacros.IsValid` _returnvalue
    (:`Is Valid`
      (`self.EnableInput` _returnvalue)
      (`self.EnableInput` (`GameplayStatics.GetPlayerController` 0))
      (`SceneComponent.SetHiddenInGame` (`self.Plane`) false true))))

(event `self.B_TriggerZone.OnComponentEndOverlap`
  (params (OverlappedComponent :type "PrimitiveComponent Object Reference") (OtherActor :type "Actor Object Reference") (OtherComp :type "PrimitiveComponent Object Reference") (OtherBodyIndex :type Integer))
  (bind _returnvalue (`GameplayStatics.GetPlayerController` 1))
  (`/Engine/EditorBlueprintResources/StandardMacros.IsValid` _returnvalue
    (:`Is Valid`
      (`self.DisableInput` _returnvalue)
      (`self.DisableInput` (`GameplayStatics.GetPlayerController` 0))
      (`SceneComponent.SetHiddenInGame` (`self.Plane`) true true))))

(event `self.trigger.OnComponentBeginOverlap`
  (params (OverlappedComponent :type "PrimitiveComponent Object Reference") (OtherActor :type "Actor Object Reference") (OtherComp :type "PrimitiveComponent Object Reference") (OtherBodyIndex :type Integer) (bFromSweep :type Boolean) (SweepResult :type "HitResult Structure (by ref)"))
  (bind _returnvalue (`GameplayStatics.GetPlayerController` 1))
  (`/Engine/EditorBlueprintResources/StandardMacros.IsValid` _returnvalue
    (:`Is Valid`
      (`self.EnableInput` _returnvalue)
      (`self.EnableInput` (`GameplayStatics.GetPlayerController` 0))
      (`ActorComponent.Activate` (`self.NS_KeyPickupArea`) false)
      (bind (_direction _colorchangespeed) (`Timeline|Timeline` :!label _label)
        (:`Update`
          (`MaterialInstanceDynamic.SetVectorParameterValue` (`self.DynamicMaterial`) "EmissiveColor" (`KismetMathLibrary.LinearColorLerp` (struct :`A` 1.0) (`self.Color`) _colorchangespeed)))))))

(event `self.trigger.OnComponentEndOverlap`
  (params (OverlappedComponent :type "PrimitiveComponent Object Reference") (OtherActor :type "Actor Object Reference") (OtherComp :type "PrimitiveComponent Object Reference") (OtherBodyIndex :type Integer))
  (bind _returnvalue (`GameplayStatics.GetPlayerController` 1))
  (`/Engine/EditorBlueprintResources/StandardMacros.IsValid` _returnvalue
    (:`Is Valid`
      (`self.DisableInput` _returnvalue)
      (`self.DisableInput` (`GameplayStatics.GetPlayerController` 0))
      (`ActorComponent.Deactivate` (`self.NS_KeyPickupArea`))
      (goto _label :!via `Reverse`))))

(event `self.ReceiveBeginPlay`
  (`SceneComponent.SetHiddenInGame` (`self.Plane`) true true)
  (`ActorComponent.Deactivate` (`self.NS_KeyPickupArea`))
  (`ActorComponent.Deactivate` (`self.NS_KeyPickup`))
  (bind _asbp_third_person_character (cast `/Game/ThirdPerson/Blueprints/BP_ThirdPersonCharacter` (`GameplayStatics.GetPlayerCharacter` 0)))
  (set `self.Player1ref` _asbp_third_person_character)
  (bind _asbp_third_person_character_2 (cast `/Game/ThirdPerson/Blueprints/BP_ThirdPersonCharacter2` (`GameplayStatics.GetPlayerCharacter` 1)))
  (set `self.Player2Ref` _asbp_third_person_character_2)
  (bind _returnvalue (`PrimitiveComponent.CreateDynamicMaterialInstance` (`self.key`) 0 "/Game/Art/Materials/MI_key.MI_key" "None"))
  (set `self.DynamicMaterial` _returnvalue)
  (bind _returnvalue_2 (`MaterialInstanceDynamic.K2_GetVectorParameterValue` (`self.DynamicMaterial`) "EmissiveColor"))
  (set `self.InitialEmissiveColor` _returnvalue_2))

(event `Key|E`
  (params (Key :type "Key Structure"))
  (:`Pressed`
    (bind _asbp_game_state (cast `/Game/ThirdPerson/Blueprints/BP_gameState` (`GameplayStatics.GetGameState`) :!label _label_2))
    (`/Game/ThirdPerson/Blueprints/BP_gameState.AddKeyToInventory` _asbp_game_state (`self.keyAd`))
    (`ActorComponent.Deactivate` (`self.NS_KeyPickupArea`))
    (`ActorComponent.Activate` (`self.NS_KeyPickup`) true)
    (`ActorComponent.K2_DestroyComponent` (`self.key`))
    (`KismetSystemLibrary.Delay` 1.0)
    (`self.K2_DestroyActor`))
  (:`Released`
    (goto _label_2)))

(event `Key|Gamepad_FaceButton_Right`
  (params (Key :type "Key Structure"))
  (:`Pressed`
    (goto _label_2))
  (:`Released`
    (goto _label_2)))

(fn `UserConstructionScript`
  (`MeshComponent.SetColorParameterValueOnMaterials` (`self.key`) "FlatColor" (`self.Color`)))