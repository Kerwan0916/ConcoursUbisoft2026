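; BP_GarageDoor is a garage door that can open and also serves as the exit that ends the game.
; The openDoor event plays a timeline that drives the door mesh's relative Z location.
; Any actor overlap checks WinConditionReached on BP_gameState and, if true, after a short delay shows the WBP_outro widget, switches to UI-only input and hides the cursor.
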(event `openDoor`
  (bind (_direction _zanim) (`Timeline|openDoorAnim`)
    (:`Update`
      (`SceneComponent.K2_SetRelativeTransform` (`self.SM_GarageDoor_01`) (`KismetMathLibrary.MakeTransform` (`KismetMathLibrary.MakeVector` 0.0 0.0 _zanim)) false false))))

(event `self.ReceiveActorBeginOverlap`
  (params (OtherActor :type "Actor Object Reference"))
  (bind _returnvalue (`GameplayStatics.GetPlayerController` 0))
  (bind _asbp_game_state (cast `/Game/ThirdPerson/Blueprints/BP_gameState` (`GameplayStatics.GetGameState`)))
  (if (== (`/Game/ThirdPerson/Blueprints/BP_gameState.bWinConditionReached` _asbp_game_state) true)
    (`KismetSystemLibrary.Delay` 1.0)
    (bind _returnvalue_2 (`|CreateWidget` "/Game/MainMenu/WBP_outro.WBP_outro_C"))
    (`UserWidget.AddToViewport` _returnvalue_2 0)
    (`WidgetBlueprintLibrary.SetInputMode_UIOnlyEx` _returnvalue null)
    (set `PlayerController.bShowMouseCursor` false _returnvalue)))

(fn `UserConstructionScript`)