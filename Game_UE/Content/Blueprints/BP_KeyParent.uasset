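; Base key pickup actor that the player collects to add a key to their owned keys.
; Overlapping the trigger enables input and shows a text prompt, and leaving reverses both.
; E or gamepad bottom face button records the key, calls PickUpItem on Player1Ref, then destroys the actor; the graph's only Player1Ref assignment is disconnected.
; The construction script tints the key meshes with a configurable color.
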(event `self.trigger.OnComponentBeginOverlap`
  (params (OverlappedComponent :type "PrimitiveComponent Object Reference") (OtherActor :type "Actor Object Reference") (OtherComp :type "PrimitiveComponent Object Reference") (OtherBodyIndex :type Integer) (bFromSweep :type Boolean) (SweepResult :type "HitResult Structure (by ref)"))
  (`self.EnableInput` (`GameplayStatics.GetPlayerController` 0))
  (`SceneComponent.SetHiddenInGame` (`self.TextRender`) false false))

(event `self.trigger.OnComponentEndOverlap`
  (params (OverlappedComponent :type "PrimitiveComponent Object Reference") (OtherActor :type "Actor Object Reference") (OtherComp :type "PrimitiveComponent Object Reference") (OtherBodyIndex :type Integer))
  (`self.DisableInput` (`GameplayStatics.GetPlayerController` 0))
  (`SceneComponent.SetHiddenInGame` (`self.TextRender`) true false))

(event `Key|E`
  (params (Key :type "Key Structure"))
  (bind _player1ref (`self.Player1Ref`))
  (:`Pressed`
    (`KismetArrayLibrary.Array_Add` (`/Game/ThirdPerson/Blueprints/BP_ThirdPersonCharacter.keyOwned` _player1ref) (`self.keyAd`) :!label _label)
    (`/Game/ThirdPerson/Blueprints/BP_ThirdPersonCharacter.PickUpItem` _player1ref (`self.ItemNumber`))
    (`self.K2_DestroyActor`)))

(event `Key|Gamepad_FaceButton_Bottom`
  (params (Key :type "Key Structure"))
  (:`Pressed`
    (goto _label)))

(fn `UserConstructionScript`
  (`MeshComponent.SetColorParameterValueOnMaterials` (`self.key`) "FlatColor" (`self.Color`))
  (`MeshComponent.SetColorParameterValueOnMaterials` (`self.r3`) "FlatColor" (`self.Color`))
  (`MeshComponent.SetColorParameterValueOnMaterials` (`self.r1`) "FlatColor" (`self.Color`))
  (`MeshComponent.SetColorParameterValueOnMaterials` (`self.r2`) "FlatColor" (`self.Color`)))