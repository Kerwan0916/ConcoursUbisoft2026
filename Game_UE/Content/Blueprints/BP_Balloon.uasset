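; BP_Balloon is a balloon prop configured entirely in its Construction Script, with no active event logic.
; A Selection switch applies a red, green or purple material instance to the Balloon component.
; It also stores a stream-seeded random yaw in RandomRotation, which spans only 0 to 1 degree and is not applied in these graphs.
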(fn `UserConstructionScript`
  (set `self.RandomRotation` (`KismetMathLibrary.MakeRotator` 0.0 0.0 (`KismetMathLibrary.RandomFloatFromStream` (`self.Stream`))))
  (switch `/Game/Blueprints/EN_BalloonColor` (`self.Selection`)
    (:`NewEnumerator0`
      (`PrimitiveComponent.SetMaterial` (`self.Balloon`) 0 "/Game/Art/Materials/MI_BalloonRed_01.MI_BalloonRed_01"))
    (:`NewEnumerator1`
      (`PrimitiveComponent.SetMaterial` (`self.Balloon`) 0 "/Game/Art/Materials/MI_BalloonGreen_01.MI_BalloonGreen_01"))
    (:`NewEnumerator2`
      (`PrimitiveComponent.SetMaterial` (`self.Balloon`) 0 "/Game/Art/Materials/MI_BalloonPurple_01.MI_BalloonPurple_01"))))