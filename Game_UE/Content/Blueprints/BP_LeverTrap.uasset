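; BP_LeverTrap is an interactable lever that opens trap doors on matching BP_Vent actors.
; Interact plays a timeline that pitches the LeverTrapDoor component between two angles.
; On every timeline update, it searches all BP_Vent actors and calls OpenTrapDoor on those whose TrapDoorValue equals the lever's ButtonValue, so the call repeats throughout the animation.
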(event `self.Interact`
  (bind (_direction _lever1) (`Timeline|Trap Door lever`)
    (:`Update`
      (`SceneComponent.K2_SetRelativeRotation` (`self.LeverTrapDoor`) (`KismetMathLibrary.RLerp` (struct :`Roll` -50.0) (struct :`Roll` 30.0) _lever1) false false)
      (bind _outactors (`GameplayStatics.GetAllActorsOfClass` "/Game/Blueprints/BP_Vent.BP_Vent_C"))
      (for _array_element _outactors
        (if (== (`/Game/Blueprints/BP_Vent.TrapDoorValue` _array_element) (`self.ButtonValue`))
          (`/Game/Blueprints/BP_Vent.OpenTrapDoor` _array_element))))))

(fn `UserConstructionScript`)