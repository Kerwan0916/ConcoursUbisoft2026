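; BP_Lever3 is an interactable lever that switches the level's lighting on and reports its activation to the game state.
; Sparks play from BeginPlay until Interact stops them and runs a timeline that rotates the lever.
; Each timeline update also requests loading of the lit streaming sublevel and unloading of its "Off" counterpart.
; On finish, it sets IsActivated and calls RegisterLeverActivate on BP_gameState.
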(event `self.Interact`
  (`ActorComponent.Deactivate` (`self.NS_Sparks`))
  (bind (_direction _lever1) (`Timeline|Timeline`)
    (:`Update`
      (`SceneComponent.K2_SetRelativeRotation` (`self.Lever3`) (`KismetMathLibrary.RLerp` (struct :`Roll` -80.0) (struct :`Roll` 80.0) _lever1) false false)
      (`GameplayStatics.LoadStreamLevel` "Lvl_Lighting_03" true)
      (`GameplayStatics.UnloadStreamLevel` "Lvl_Lighting_03_Off"))
    (:`Finished`
      (set `self.IsActivated` true)
      (bind _asbp_game_state (cast `/Game/ThirdPerson/Blueprints/BP_gameState` (`GameplayStatics.GetGameState`)))
      (`/Game/ThirdPerson/Blueprints/BP_gameState.RegisterLeverActivate` _asbp_game_state))))

(event `self.ReceiveBeginPlay`
  (`ActorComponent.Activate` (`self.NS_Sparks`) false))

(fn `UserConstructionScript`)