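; BP_CyanDoor is a door actor that swings open when the third-person character presses while inside its trigger box.
; Box overlaps set or clear an Inside flag for BP_ThirdPersonCharacter.
; On overlap begin, and every Tick while Inside, it reads the character's PressCheck from the overlap's OtherActor.
; When true, the DoorAnim timeline plays, scaling its track by 90 degrees to set LeftDoor's yaw, with no closing logic.
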(event `self.ReceiveTick`
  (params (DeltaSeconds :type "Float (single-precision)"))
  (if (`self.Inside`)
    (bind _asbp_third_person_character (cast `/Game/ThirdPerson/Blueprints/BP_ThirdPersonCharacter` (stale `self.Box.OnComponentBeginOverlap` OtherActor) :!label _label))
    (set `self.Inside` true)
    (if (`/Game/ThirdPerson/Blueprints/BP_ThirdPersonCharacter.PressCheck` _asbp_third_person_character)
      (bind (_direction _newtrack_0) (`Timeline|DoorAnim`)
        (:`Update`
          (`SceneComponent.K2_SetRelativeRotation` (`self.LeftDoor`) (`KismetMathLibrary.MakeRotator` 0.0 0.0 (* _newtrack_0 90.0)) false false))))))

(event `self.Box.OnComponentBeginOverlap`
  (params (OverlappedComponent :type "PrimitiveComponent Object Reference") (OtherActor :type "Actor Object Reference") (OtherComp :type "PrimitiveComponent Object Reference") (OtherBodyIndex :type Integer) (bFromSweep :type Boolean) (SweepResult :type "HitResult Structure (by ref)"))
  (goto _label))

(event `self.Box.OnComponentEndOverlap`
  (params (OverlappedComponent :type "PrimitiveComponent Object Reference") (OtherActor :type "Actor Object Reference") (OtherComp :type "PrimitiveComponent Object Reference") (OtherBodyIndex :type Integer))
  (cast `/Game/ThirdPerson/Blueprints/BP_ThirdPersonCharacter` OtherActor)
  (set `self.Inside` false))

(fn `UserConstructionScript`)