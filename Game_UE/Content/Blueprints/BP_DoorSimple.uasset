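; BP_DoorSimple is a double door that swings open when a pawn overlaps it.
; A single timeline drives the yaw of both leaves in mirrored directions, playing to open and reversing to close.
; Any actor ending overlap triggers closing, as only the begin overlap checks for a pawn.
; The construction script assigns a configurable material to each leaf by slot name.
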(event `self.ReceiveActorBeginOverlap`
  (params (OtherActor :type "Actor Object Reference"))
  (cast `Pawn` OtherActor)
  (`self.Open door`))

(event `self.ReceiveActorEndOverlap`
  (params (OtherActor :type "Actor Object Reference"))
  (`self.Close door`))

(event `Open door`
  (bind (_direction _newtrack_0) (`Timeline|DoorAnim` :!label _label)
    (:`Update`
      (`SceneComponent.K2_SetRelativeRotation` (`self.LeftDoor`) (`KismetMathLibrary.MakeRotator` 0.0 0.0 _newtrack_0) false false)
      (`SceneComponent.K2_SetRelativeRotation` (`self.RightDoor`) (`KismetMathLibrary.MakeRotator` 0.0 0.0 (* _newtrack_0 -1.0)) false false))))

(event `Close door`
  (goto _label :!via `Reverse`))

(fn `UserConstructionScript`
  (`PrimitiveComponent.SetMaterialByName` (`self.LeftDoor`) "standardSurface1" (`self.Material_LeftDoor`))
  (`PrimitiveComponent.SetMaterialByName` (`self.RightDoor`) "standardSurface1" (`self.Material_RightDoor`)))