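; Parent Blueprint for a key-locked double door that opens when an overlapping Character's required key is owned.
; Overlap checks KeyDoor against KeysOwned on the BP_gameState actor, then a one-time flag gates both opening and the 2D sound.
; The DoorAnim timeline yaws both leaves in opposite directions, while CloseDoor runs on end overlap but is empty.
; The construction script applies separate materials to each leaf.
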(event `self.ReceiveActorBeginOverlap`
  (params (OtherActor :type "Actor Object Reference"))
  (cast `Character` OtherActor)
  (bind _returnvalue (`GameplayStatics.GetActorOfClass` "/Game/ThirdPerson/Blueprints/BP_gameState.BP_gameState_C"))
  (if (`KismetArrayLibrary.Array_Contains` (`/Game/ThirdPerson/Blueprints/BP_gameState.keysOwned` _returnvalue) (`self.keyDoor`))
    (if (not (`self.PlayDoorSFX`))
      (`self.Open door`)
      ;[0.3271 0.1615 1 0.5] SFX ROOM DOOR OPEN
      (`GameplayStatics.PlaySound2D` "/Game/Sound/World_Objects/SFX_DOOR_ROOM_OPEN_01.SFX_DOOR_ROOM_OPEN_01" 1.0 1.0 0.0 null null)
      (set `self.PlayDoorSFX` true))))

(event `self.ReceiveActorEndOverlap`
  (params (OtherActor :type "Actor Object Reference"))
  (`self.Close door`))

(event `Open door`
  (bind (_direction _newtrack_0) (`Timeline|DoorAnim`)
    (:`Update`
      (`SceneComponent.K2_SetRelativeRotation` (`self.LeftDoor`) (`KismetMathLibrary.MakeRotator` 0.0 0.0 _newtrack_0) false false)
      (`SceneComponent.K2_SetRelativeRotation` (`self.RightDoor`) (`KismetMathLibrary.MakeRotator` 0.0 0.0 (* _newtrack_0 -1.0)) false false))))

(event `Close door`)

(fn `UserConstructionScript`
  (`PrimitiveComponent.SetMaterialByName` (`self.LeftDoor`) "standardSurface1" (`self.Material_LeftDoor`))
  (`PrimitiveComponent.SetMaterialByName` (`self.RightDoor`) "standardSurface1" (`self.Material_RightDoor`)))